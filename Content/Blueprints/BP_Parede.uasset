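; BP_Parede is a wall actor that can spawn a random power-up at its Cube's location when Drop is called.
; Drop makes a chain of separate random rolls, trying bomb first, then fire, then speed, and may spawn nothing.
; The speed check ANDs two independent rolls rather than testing one value against a range.
; The event graph and construction script are empty, so Drop relies on an external caller.
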(fn `Drop`
  (bind _returnvalue (`KismetMathLibrary.RandomFloatInRange` 0.0 100.0))
  (bind _returnvalue_2 (`KismetMathLibrary.Conv_VectorToTransform` (`SceneComponent.K2_GetComponentLocation` (`self.Cube`))))
  (if (< _returnvalue 15.0)
    (`|SpawnActorFromClass` "/Game/Blueprints/BP_PowerUPBomba.BP_PowerUPBomba_C" _returnvalue_2 "Undefined" "OverrideRootScale" null null)
    (elif (> _returnvalue 85.0)
      (`|SpawnActorFromClass` "/Game/Blueprints/BP_PowerUPFire.BP_PowerUPFire_C" _returnvalue_2 "Undefined" "OverrideRootScale" null null)
      (elif (and (< _returnvalue 80.0) (> _returnvalue 45.0))
        (`|SpawnActorFromClass` "/Game/Blueprints/BP_PowerUPVelocidade.BP_PowerUPVelocidade_C" _returnvalue_2 "Undefined" "OverrideRootScale" null null)))))

(fn `UserConstructionScript`)