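; BP_Bomba1 is a timed bomb in a two-player game that kills BP_Jogador2 and breaks walls within its blast sphere.
; On BeginPlay it sizes Sphere1 from the game instance's Bomba2Range, waits briefly, then decrements Bombas1 on every BP_Jogador2.
; Overlapping walls call Drop and are destroyed; hitting BP_Jogador2 records Player 1's win and opens the victory level.
; The bomb then destroys itself; a disconnected branch for hitting BP_Jogador never runs.
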(event `self.ReceiveBeginPlay`
  (bind _gameinstance (`self.GameInstance`))
  (bind _asnew_game_instance (cast `/Game/Blueprints/NewGameInstance` (`GameplayStatics.GetGameInstance`)))
  (bind _output_get (set `self.GameInstance` _asnew_game_instance))
  (`SphereComponent.SetSphereRadius` (`self.Sphere1`) (`/Game/Blueprints/NewGameInstance.Bomba2Range` _output_get) true)
  (`KismetSystemLibrary.Delay` 1.0)
  (bind _outactors (`GameplayStatics.GetAllActorsOfClass` "/Game/Blueprints/BP_Jogador2.BP_Jogador2_C"))
  (for _array_element _outactors
    (`/Engine/EditorBlueprintResources/StandardMacros.DecrementInt` (`/Game/Blueprints/BP_Jogador2.Bombas1` _array_element)))
  (bind _output_get_2 (set `self.Overllaping` (`PrimitiveComponent.GetOverlappingActors` (`self.Sphere1`) null)))
  (for _array_element_2 _output_get_2
    (bind _returnvalue (`GameplayStatics.GetObjectClass` _array_element_2))
    (if (== _returnvalue "/Game/Blueprints/BP_Jogador2.BP_Jogador2_C")
      (`self.K2_DestroyActor` _array_element_2)
      (set `/Game/Blueprints/NewGameInstance.Jogador1Win` (+ (`/Game/Blueprints/NewGameInstance.Jogador1Win` _gameinstance) 1.0) _gameinstance)
      (set `/Game/Blueprints/NewGameInstance.Jogador2Lose` (+ (`/Game/Blueprints/NewGameInstance.Jogador2Lose` _gameinstance) 1.0) _gameinstance)
      (`GameplayStatics.OpenLevel` "VitoriaJogador1")
      (elif (== _returnvalue "/Game/Blueprints/BP_Parede.BP_Parede_C")
        (bind _asbp_parede (cast `/Game/Blueprints/BP_Parede` _array_element_2))
        (`/Game/Blueprints/BP_Parede.Drop` _asbp_parede)
        (`self.K2_DestroyActor` _array_element_2))))
  (`self.K2_DestroyActor`))

(fn `UserConstructionScript`)