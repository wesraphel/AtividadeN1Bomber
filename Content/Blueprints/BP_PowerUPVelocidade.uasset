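; BP_PowerUPVelocidade is a speed power-up pickup for the two player characters.
; When its Box begins overlapping a BP_Jogador or BP_Jogador2, it adds a fixed bonus to that player's Velocidade and then destroys itself.
; The player is identified by exact class comparison followed by a cast, with a separate branch per player class, and other actors are ignored.
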(event `self.Box.OnComponentBeginOverlap`
  (params (OverlappedComponent :type "PrimitiveComponent Object Reference") (OtherActor :type "Actor Object Reference") (OtherComp :type "PrimitiveComponent Object Reference") (OtherBodyIndex :type Integer) (bFromSweep :type Boolean) (SweepResult :type "HitResult Structure (by ref)"))
  (bind _returnvalue (`GameplayStatics.GetObjectClass` OtherActor))
  (if (== _returnvalue "/Game/Blueprints/BP_Jogador.BP_Jogador_C")
    (bind _asbp_jogador (cast `/Game/Blueprints/BP_Jogador` OtherActor))
    (set `/Game/Blueprints/BP_Jogador.Velocidade` (+ (`/Game/Blueprints/BP_Jogador.Velocidade` _asbp_jogador) 80.0) _asbp_jogador)
    (`self.K2_DestroyActor` :!label _label)
    (elif (== _returnvalue "/Game/Blueprints/BP_Jogador2.BP_Jogador2_C")
      (bind _asbp_jogador_2 (cast `/Game/Blueprints/BP_Jogador2` OtherActor))
      (set `/Game/Blueprints/BP_Jogador2.Velocidade` (+ (`/Game/Blueprints/BP_Jogador2.Velocidade` _asbp_jogador_2) 80.0) _asbp_jogador_2)
      (goto _label))))

(fn `UserConstructionScript`)