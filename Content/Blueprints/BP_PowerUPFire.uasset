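; BP_PowerUPFire is a fire power-up pickup that increases the bomb range of the player who collects it.
; When its Box component is overlapped, it checks whether the actor's class is exactly BP_Jogador or BP_Jogador2.
; It then adds a fixed amount to that player's range variable in NewGameInstance (Bomba1Range or Bomba2Range) and destroys itself.
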(event `self.Box.OnComponentBeginOverlap`
  (params (OverlappedComponent :type "PrimitiveComponent Object Reference") (OtherActor :type "Actor Object Reference") (OtherComp :type "PrimitiveComponent Object Reference") (OtherBodyIndex :type Integer) (bFromSweep :type Boolean) (SweepResult :type "HitResult Structure (by ref)"))
  (bind _returnvalue (`GameplayStatics.GetObjectClass` OtherActor))
  (bind _returnvalue_2 (`GameplayStatics.GetGameInstance`))
  (if (== _returnvalue "/Game/Blueprints/BP_Jogador.BP_Jogador_C")
    (bind _asnew_game_instance (cast `/Game/Blueprints/NewGameInstance` _returnvalue_2))
    (set `/Game/Blueprints/NewGameInstance.Bomba1Range` (+ (`/Game/Blueprints/NewGameInstance.Bomba1Range` _asnew_game_instance) 40.0) _asnew_game_instance)
    (`self.K2_DestroyActor` :!label _label)
    (elif (== _returnvalue "/Game/Blueprints/BP_Jogador2.BP_Jogador2_C")
      (bind _asnew_game_instance_2 (cast `/Game/Blueprints/NewGameInstance` _returnvalue_2))
      (set `/Game/Blueprints/NewGameInstance.Bomba2Range` (+ (`/Game/Blueprints/NewGameInstance.Bomba2Range` _asnew_game_instance_2) 40.0) _asnew_game_instance_2)
      (goto _label))))

(fn `UserConstructionScript`)