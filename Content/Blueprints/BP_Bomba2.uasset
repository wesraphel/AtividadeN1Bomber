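; BP_Bomba2 is a timed bomb in a two-player game that destroys players and walls within its blast sphere.
; After a short delay from BeginPlay, it checks the actors overlapping Sphere1 by class, then destroys itself.
; A hit on BP_Jogador or BP_Jogador2 updates win and loss counters in the GameInstance and opens the other player's victory level.
; BP_Parede walls caught in the sphere are simply destroyed.
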(event `self.ReceiveBeginPlay`
  (bind _gameinstance (`self.GameInstance`))
  (bind _gameinstance_2 (`self.GameInstance`))
  (`KismetSystemLibrary.Delay` 1.0)
  (bind _output_get (set `self.Overllaping` (`PrimitiveComponent.GetOverlappingActors` (`self.Sphere1`) null)))
  (for _array_element _output_get
    (bind _returnvalue (`GameplayStatics.GetObjectClass` _array_element))
    (if (== _returnvalue "/Game/Blueprints/BP_Jogador2.BP_Jogador2_C")
      (`self.K2_DestroyActor` _array_element)
      (set `/Game/Blueprints/NewGameInstance.Jogador1Win` (+ (`/Game/Blueprints/NewGameInstance.Jogador1Win` _gameinstance_2) 1.0) _gameinstance_2)
      (set `/Game/Blueprints/NewGameInstance.Jogador2Lose` (+ (`/Game/Blueprints/NewGameInstance.Jogador2Lose` _gameinstance_2) 1.0) _gameinstance_2)
      (`GameplayStatics.OpenLevel` "VitoriaJogador1")
      (elif (== _returnvalue "/Game/Blueprints/BP_Jogador.BP_Jogador_C")
        (`self.K2_DestroyActor` _array_element)
        (set `/Game/Blueprints/NewGameInstance.Jogador2Win` (+ (`/Game/Blueprints/NewGameInstance.Jogador2Win` _gameinstance) 1.0) _gameinstance)
        (set `/Game/Blueprints/NewGameInstance.Jogador1Lose` (+ (`/Game/Blueprints/NewGameInstance.Jogador1Lose` _gameinstance) 1.0) _gameinstance)
        (`GameplayStatics.OpenLevel` "VitoriaJogador2")
        (elif (== _returnvalue "/Game/Blueprints/BP_Parede.BP_Parede_C")
          (cast `/Game/Blueprints/BP_Parede` _array_element)
          (`self.K2_DestroyActor` _array_element)))))
  (`self.K2_DestroyActor`))

(fn `UserConstructionScript`)