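; BP_Jogador2 is a player-controlled Blueprint, apparently for player 2, that moves a physics cube and drops bombs.
; LEFTRIGHT and UPDOWN axes apply acceleration forces along the cube's right and forward vectors.
; Tick clamps the full velocity vector when horizontal speed exceeds Velocidade.
; Enter spawns BP_Bomba1 above the cube and increments Bombas1, unless it equals MaxBombas1.
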(event `self.ReceiveTick`
  (params (DeltaSeconds :type "Float (single-precision)"))
  (bind (_returnvalue_x _returnvalue_y) (`KismetMathLibrary.BreakVector` (`SceneComponent.GetComponentVelocity` (`self.Cube`))))
  (if (> (`KismetMathLibrary.VSize` (`KismetMathLibrary.MakeVector` _returnvalue_x _returnvalue_y)) (`self.Velocidade`))
    (`PrimitiveComponent.SetPhysicsLinearVelocity` (`self.Cube`) (`KismetMathLibrary.ClampVectorSize` (`SceneComponent.GetComponentVelocity` (`self.Cube`)) 0.0 (`self.Velocidade`)) false "None")))

(event `InputAxis|LEFTRIGHT  `
  (params (AxisValue :type "Float (single-precision)"))
  (`PrimitiveComponent.AddForce` (`self.Cube`) (* (`SceneComponent.GetRightVector` (`self.Cube`)) (* AxisValue (`self.Forca`))) "None" true))

(event `InputAxis|UPDOWN`
  (params (AxisValue :type "Float (single-precision)"))
  (`PrimitiveComponent.AddForce` (`self.Cube`) (* (`SceneComponent.GetForwardVector` (`self.Cube`)) (* (`self.Forca`) AxisValue)) "None" true))

(event `Key|Enter`
  (params (Key :type "Key Structure"))
  (:`Pressed`
    (if (!= (`self.Bombas1`) (`self.MaxBombas1`))
      (`|SpawnActorFromClass` "/Game/Blueprints/BP_Bomba1.BP_Bomba1_C" (`KismetMathLibrary.Conv_VectorToTransform` (`KismetMathLibrary.MakeVector` (.x (`SceneComponent.K2_GetComponentLocation` (`self.Cube`))) (.y (`SceneComponent.K2_GetComponentLocation` (`self.Cube`))) (+ (.z (`SceneComponent.K2_GetComponentLocation` (`self.Cube`))) 200.0))) "Undefined" "OverrideRootScale" null null)
      (`/Engine/EditorBlueprintResources/StandardMacros.IncrementInt` (`self.Bombas1`)))))

(fn `UserConstructionScript`)